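; BP_Spline_Chain is a dungeon prop that builds a chain along an editable spline out of repeated spline mesh segments.
; The construction script divides the spline length by MeshLength and adds one collision-enabled spline mesh component per step.
; Each segment takes its positions and tangents by distance along the spline, with tangents clamped to MeshLength and ends pushed slightly forward to overlap the next.
; The event graph is empty, so no runtime logic runs.
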(fn `UserConstructionScript`
  (bind _meshlength (`self.MeshLength`))
  (bind _spline (`self.Spline`))
  (for _index (range (+ (`KismetMathLibrary.FTrunc` (/ (`SplineComponent.GetSplineLength` (`self.Spline`)) (`self.MeshLength`))) 1))
    (bind _returnvalue (`AddComponent|NODE_AddSplineMeshComponent-0`))
    (bind _returnvalue_2 (* _index (`self.MeshLength`)))
    (bind _returnvalue_3 (* (+ _index 1) (`self.MeshLength`)))
    (`SplineMeshComponent.SetStartAndEnd` _returnvalue (`SplineComponent.GetLocationAtDistanceAlongSpline` (`self.Spline`) _returnvalue_2 "Local") (`KismetMathLibrary.ClampVectorSize` (`SplineComponent.GetTangentAtDistanceAlongSpline` _spline _returnvalue_2 "Local") 0.0 _meshlength) (`SplineComponent.GetLocationAtDistanceAlongSpline` (`self.Spline`) (+ _returnvalue_3 6.5) "Local") (`KismetMathLibrary.ClampVectorSize` (`SplineComponent.GetTangentAtDistanceAlongSpline` _spline _returnvalue_3 "Local") 0.0 _meshlength) true)
    (`PrimitiveComponent.SetCollisionEnabled` _returnvalue "QueryAndPhysics")))