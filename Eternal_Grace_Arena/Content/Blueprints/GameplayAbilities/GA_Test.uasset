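; GA_Test is a gameplay ability that appears to be a test, pushing its avatar forward while playing an interact montage.
; On a successful commit it applies constant-force root motion along the actor's forward vector, then plays AM_Interact and waits once for AttackEvent, with no handler wired.
; The ability ends when the montage finishes or stops, or when commit fails, with debug logs throughout.
; An unconnected fragment would apply a gameplay effect to a target.
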(event `self.K2_ActivateAbility`
  (bind _returnvalue (`self.K2_CommitAbility`))
  (if _returnvalue
    (`KismetSystemLibrary.LogString` "yeah")
    (`AbilityTask_ApplyRootMotionConstantForce.ApplyRootMotionConstantForce` "None" (`Actor.GetActorForwardVector` (`self.GetAvatarActorFromActorInfo`)) 250.0 25.0 false null "MaintainLastRootMotionVelocity"
      (:`then`
        (`AbilityTask_PlayMontageAndWait.CreatePlayMontageAndWaitProxy` "None" "/Game/Animations/PlayerAnimations/Interactions/AM_Interact.AM_Interact"
          (:`then`
            (`AbilityTask_WaitGameplayEvent.WaitGameplayEvent` (struct :`TagName` "AttackEvent") null true))
          (:`OnCompleted`
            (`self.K2_EndAbility` :!label _label))
          (:`OnBlendOut`
            (goto _label))
          (:`OnInterrupted`
            (goto _label))
          (:`OnCancelled`
            (goto _label)))))
    (else
      (`KismetSystemLibrary.LogString` "Hello")
      (`self.K2_EndAbility`))))

(event `self.K2_OnEndAbility`
  (params (bWasCancelled :type Boolean))
  (`KismetSystemLibrary.LogString` "finish"))