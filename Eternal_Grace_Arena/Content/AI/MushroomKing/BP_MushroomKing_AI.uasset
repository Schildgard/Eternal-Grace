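; AI controller for the Mushroom King enemy that drives it through the BT_MushroomKing behavior tree.
; On BeginPlay it starts the tree, then seeds the blackboard with the first player character and the controller's own location as StartingPosition.
; An unconnected branch that would copy the arena enemy's IsAggro flag into spottedPlayer never runs.
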(event `self.ReceiveBeginPlay`
  (bind _returnvalue (`AIBlueprintHelperLibrary.GetBlackboard` null))
  (`self.RunBehaviorTree` "/Game/AI/MushroomKing/BT_MushroomKing.BT_MushroomKing")
  (`BlackboardComponent.SetValueAsObject` _returnvalue "Player" (`GameplayStatics.GetPlayerCharacter` 0))
  (`BlackboardComponent.SetValueAsVector` _returnvalue "StartingPosition" (`self.K2_GetActorLocation`)))

(fn `UserConstructionScript`)