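; AI controller for the mage boss that starts its behavior tree when play begins.
; After running BT_MageBoss, it seeds the blackboard with the player character and the controller's own location as StartingPosition.
; An unconnected block that would copy the arena enemy's IsAggro flag into spottedPlayer never runs, and Tick is unused.
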(event `self.ReceiveBeginPlay`
  (bind _returnvalue (`AIBlueprintHelperLibrary.GetBlackboard` null))
  (`self.RunBehaviorTree` "/Game/AI/MageBoss/BT_MageBoss.BT_MageBoss")
  (`BlackboardComponent.SetValueAsObject` _returnvalue "Player" (`GameplayStatics.GetPlayerCharacter` 0))
  (`BlackboardComponent.SetValueAsVector` _returnvalue "StartingPosition" (`self.K2_GetActorLocation`)))

(fn `UserConstructionScript`)